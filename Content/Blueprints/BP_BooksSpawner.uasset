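; Procedural prop actor that builds a row or stack of randomly chosen book meshes in its construction script when switched on.
; The base mesh component holds the first book, and each further book is added as a static mesh component offset from the previous one using bounding-box extents.
; Stacks lay books flat with random yaw, while rows share a lean angle, with height compensation and random depth jitter.
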(fn ConstructionScript
  (bind _xoffset (Variables|Default|GetXOffset))
  (bind _staticmesh (Variables|Components|GetStaticMesh))
  (bind _staticmesh_2 (Variables|Components|GetStaticMesh))
  (bind _staticmesh_3 (Variables|Components|GetStaticMesh))
  (bind _staticmesh_4 (Variables|/Script/Engine.StaticMeshComponent|GetStaticMesh _staticmesh))
  (bind _staticmesh_5 (Variables|/Script/Engine.StaticMeshComponent|GetStaticMesh _staticmesh_2))
  (bind _staticmesh_6 (Variables|/Script/Engine.StaticMeshComponent|GetStaticMesh _staticmesh_3))
  (bind _returnvalue (StaticMesh|GetBoundingBox _staticmesh_4))
  (bind _returnvalue_2 (StaticMesh|GetBoundingBox _staticmesh_5))
  (bind _returnvalue_3 (StaticMesh|GetBoundingBox _staticmesh_6))
  (if (Variables|Default|GetbIsOn?)
    (Components|StaticMesh|SetStaticMesh (Variables|Components|GetStaticMesh) (.OutItem (Utilities|Array|Random (Variables|Default|GetBooksMeshes))))
    (if (Variables|Default|GetbAreStacked?)
      ;[0 0.3512 1 0.5] Z Axis
      (Transformation|SetRelativeTransform (Variables|Components|GetStaticMesh) (Math|Transform|MakeTransform (+ (Math|Vector|Lerp(Vector) (Math|Vector|RotateVectorAroundAxis (.min _returnvalue) -9e+01 "0.000000,1.000000,0.000000") (+ (Variables|/Script/Engine.SceneComponent|GetRelativeLocation (Variables|Components|GetStaticMesh)) (Math|Vector|RotateVectorAroundAxis (.max _returnvalue) -9e+01 "0.000000,1.000000,0.000000")) 0.5) (Math|Vector|MakeVector 0.0 0.0 (.X (Class|KismetMathLibrary|BreakVector3f (/ (- (.max _returnvalue_2) (.min _returnvalue_2)) 2))))) "-90.000000,0.000000,0.000000" "1.000000,1.000000,1.000000") false false)
      (Variables|Components|SetPreviousBook (Variables|Components|GetStaticMesh))
      (for _index (range 2 (Variables|Default|GetBooksNum))
        (Variables|Default|SetNextBook (.OutItem (Utilities|Array|Random (Variables|Default|GetBooksMeshes))))
        (bind (_verticaloffset _rotation) (CallFunction|VerticalOffset))
        (CallFunction|GenerateBook _verticaloffset _rotation))
      (else
        ;[1 0.057 0 0.5] X Axis
        (Transformation|SetRelativeTransform (Variables|Components|GetStaticMesh) (Math|Transform|MakeTransform (Math|Vector|MakeVector 0.0 0.0 (* (Math|Float|Absolute(Float) (Math|Trig|Sin(Degrees) (Variables|Default|GetLeanRotation))) (.X (Math|Vector|BreakVector (/ (- (.max _returnvalue_3) (.min _returnvalue_3)) 2))))) (Math|Rotator|MakeRotator 0.0 (* (Variables|Default|GetLeanRotation) -1) 0.0) "1.000000,1.000000,1.000000") false false)
        (Variables|Components|SetPreviousBook (Variables|Components|GetStaticMesh))
        (for _index_2 (range 2 (Variables|Default|GetBooksNum))
          (Variables|Default|SetNextBook (.OutItem (Utilities|Array|Random (Variables|Default|GetBooksMeshes))))
          (bind (_horizontaloffset _rotation_2) (CallFunction|HorizontalOffset _xoffset _xoffset))
          (CallFunction|GenerateBook _horizontaloffset _rotation_2))))))

(fn HorizontalOffset
  (params (MinXOffset :type Float%20%28double-precision%29) (MaxXOffset :type Float%20%28double-precision%29))
  (bind _nextbook (Variables|Default|GetNextBook))
  (bind _previousbook (Variables|Components|GetPreviousBook))
  (bind _returnvalue (StaticMesh|GetBoundingBox _nextbook))
  (bind _staticmesh (Variables|/Script/Engine.StaticMeshComponent|GetStaticMesh _previousbook))
  (bind _returnvalue_2 (StaticMesh|GetBoundingBox _staticmesh))
  (bind _returnvalue_3 (- (.max _returnvalue) (.min _returnvalue)))
  (bind _returnvalue_4 (/ _returnvalue_3 2))
  (return (Math|Vector|MakeVector (.x (+ (+ (/ (- (.max _returnvalue_2) (.min _returnvalue_2)) 2) _returnvalue_4) (Math|Vector|MakeVector (+ (.x (Variables|/Script/Engine.SceneComponent|GetRelativeLocation _previousbook)) (Math|Random|RandomFloatinRange MinXOffset MaxXOffset)) 0.0 0.0))) (Math|Random|RandomFloatinRange 0.0 (Variables|Default|GetYOffset)) (Math|Float|Absolute(Float) (* (.X (Math|Vector|BreakVector _returnvalue_4)) (Math|Trig|Sin(Degrees) (Variables|Default|GetLeanRotation))))) (Math|Rotator|MakeRotator 0.0 (* (Variables|Default|GetLeanRotation) -1) 0.0)))

(fn VerticalOffset
  (bind _previousbook (Variables|Components|GetPreviousBook))
  (bind _nextbook (Variables|Default|GetNextBook))
  (bind _stackrotation (Variables|Default|GetStackRotation))
  (bind _returnvalue (StaticMesh|GetBoundingBox _nextbook))
  (bind _staticmesh (Variables|/Script/Engine.StaticMeshComponent|GetStaticMesh _previousbook))
  (bind _returnvalue_2 (StaticMesh|GetBoundingBox _staticmesh))
  (bind _returnvalue_3 (- (.max _returnvalue) (.min _returnvalue)))
  (bind _returnvalue_4 (- (.max _returnvalue_2) (.min _returnvalue_2)))
  (bind _returnvalue_5 (/ _returnvalue_3 2))
  (bind (_x _y _z) (Class|KismetMathLibrary|BreakVector3f _returnvalue_5))
  (bind _returnvalue_6 (/ _returnvalue_4 2))
  (bind (_x_2 _y_2 _z_2) (Class|KismetMathLibrary|BreakVector3f _returnvalue_6))
  (return (+ (+ (Variables|/Script/Engine.SceneComponent|GetRelativeLocation (Variables|Components|GetPreviousBook)) (Math|Vector|MakeVector (* _z -1.0) 0.0 _x)) (Math|Vector|MakeVector _z_2 0.0 _x_2)) (Math|Rotator|MakeRotator 0.0 -9e+01 (Math|Random|RandomFloatinRange (* _stackrotation -1.0) _stackrotation))))

(fn GenerateBook
  (params (Offset :type Vector) (Rotation :type Rotator))
  (bind _returnvalue (AddComponent|AddStaticMeshComponent false (Math|Transform|MakeTransform Offset Rotation "1.000000,1.000000,1.000000")))
  (bind _output_get (Variables|Components|SetPreviousBook _returnvalue))
  (Components|StaticMesh|SetStaticMesh _output_get (Variables|Default|GetNextBook))
  (Utilities|Array|Add (Variables|Default|GetSpawnedBooks) _returnvalue))